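; Game mode for a round-based zombie survival game that creates the main HUD widget and runs an endless wave loop.
; Each round sets a zombie total (fixed early, then scaled by round number) and drops an ammo crate every fifth round.
; A looping timer triggers random spawners while limiting concurrent zombies.
; CheckIfRoundEnd starts the next round once all are spawned and none remain.
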(event Custom|SpawnAmmo
  ;[0.15 0.15 0.15 0.5] Spawn Ammo Crate
  (Game|SpawnActorfromClass "/Game/_Game/Blueprints/BP_AmmoPickup.BP_AmmoPickup_C" (Math|Transform|MakeTransform (Utilities|Array|Get(acopy) (Variables|Default|GetAmmoCrateSpawn) (Math|Random|RandomInteger 4)) "0, 0, 0" "1.000000,1.000000,1.000000") "Undefined" "MultiplyWithRoot" 0 0))

(event Custom|IncreaseRound
  ;[0.15 0.15 0.15 0.5] Increment Round
  (Math|Integer|IncrementInt (Variables|Default|GetCurrentRound)
    (:%20%20
      (Utilities|FlowControl|Delay (Variables|Default|GetTime_Between_Round))
      (bind _foundwidgets (Widget|GetAllWidgetsOfClass "/Game/_Game/Widgets/MainWidget_W.MainWidget_W_C" true))
      (Default|IncreaseRound (Utilities|Array|Get(acopy) _foundwidgets))
      (CallFunction|StartRound))))

(event Custom|StartRound
  (bind _currentround (Variables|Default|GetCurrentRound))
  ;[0.15 0.15 0.15 0.5] Round logic
  (Variables|Default|SetTotal_Zombies_In_Round (Math|Integer|SelectInt (Math|Float|Round (* (* (Variables|Default|GetCurrentRound) 0.15) (Variables|Default|GetMax_Zombies_In_Level))) (Math|Integer|SelectInt 6 9 (== _currentround 1)) (> _currentround 2)))
  (if (== (Math|Integer|%(Integer) (Variables|Default|GetCurrentRound) 5) 0)
    (CallFunction|SpawnAmmo))
  (Utilities|FlowControl|Delay 0.2)
  (bind _returnvalue (Utilities|Time|SetTimerbyEvent (delegate Custom|SpawnZombie) (Variables|Default|GetTime_Between_Spawn) true)))

(event Custom|SpawnZombie
  ;[0.15 0.15 0.15 0.5] Round logic
  (if (< (Variables|Default|GetZombieSpawned) (Variables|Default|GetTotal_Zombies_In_Round))
    (if (<= (Variables|Default|GetZombiesLeft) (Variables|Default|GetMax_Zombies_In_Level))
      (CallFunction|Spawn)
      (Math|Integer|IncrementInt (Variables|Default|GetZombieSpawned)
        (:%20%20
          (Math|Integer|IncrementInt (Variables|Default|GetZombiesLeft)))))
    (else
      (Utilities|Time|ClearandInvalidateTimerbyHandle (stale Custom|StartRound _returnvalue)))))

(event Custom|CheckIfRoundEnd
  ;[0.15 0.15 0.15 0.5] Round logic
  (Utilities|FlowControl|Delay 0.1)
  (if (and (>= (Variables|Default|GetZombieSpawned) (Variables|Default|GetTotal_Zombies_In_Round)) (== (Variables|Default|GetZombiesLeft) 0))
    (Variables|Default|SetZombieSpawned 0)
    (CallFunction|IncreaseRound)
    (Utilities|Time|ClearandInvalidateTimerbyHandle (stale Custom|StartRound _returnvalue))))

(event EventBeginPlay
  (bind _returnvalue (UserInterface|CreateWidget "/Game/_Game/Widgets/MainWidget_W.MainWidget_W_C"))
  (bind _output_get (Variables|Default|SetMainWid _returnvalue))
  (UserInterface|Viewport|AddtoViewport _output_get 0)
  (CallFunction|IncreaseRound))

(fn ConstructionScript)

(fn Spawn
  (bind _outactors (Actor|GetAllActorsOfClass "/Game/_Game/Blueprints/BP_ZombieSpawner.BP_ZombieSpawner_C"))
  (Default|Spawn (Utilities|Array|Get(acopy) _outactors (Math|Random|RandomInteger 6))))