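; Player health component that tracks current health against a maximum for damage and recovery.
; HealthDamage subtracts a clamped amount, plays the heartbeat animation on the first top-level MainWidget_W, and returns whether health has reached zero.
; HealthRecover adds a clamped amount without touching the UI.
; Both event graph events are disabled, so all logic runs only when these functions are called.
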(event EventBeginPlay)

(event EventTick
  (params (DeltaSeconds :type Float%20%28single-precision%29)))

(fn HealthDamage
  (params (Amount :type Float%20%28double-precision%29))
  (bind _output_get (Variables|Default|SetHealthCurrent (Math|Float|Clamp(Float) (- (Variables|Default|GetHealthCurrent) Amount) 0.0 (Variables|Default|GetHealthMax))))
  (bind _foundwidgets (Widget|GetAllWidgetsOfClass "/Game/_Game/Widgets/MainWidget_W.MainWidget_W_C" true))
  (Default|HeartBeatAnim (Utilities|Array|Get(acopy) _foundwidgets))
  (return (<= _output_get 0.0)))

(fn HealthRecover
  (params (Amount :type Float%20%28double-precision%29))
  (Variables|Default|SetHealthCurrent (Math|Float|Clamp(Float) (+ (Variables|Default|GetHealthCurrent) Amount) 0.0 (Variables|Default|GetHealthMax))))